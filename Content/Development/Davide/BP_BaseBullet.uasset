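; BP_BaseBullet is a base bullet actor that detects hits and destroys itself one second after spawning.
; A looping 0.1-second timer runs a Visibility line trace along the forward axis, spanning HitDetectionLine ahead of and behind the bullet and ignoring its owner.
; Hit actors implementing IF_ShotReaction receive ShotReactionMessage with the bullet's owner, then the bullet is destroyed.
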(event `self.ReceiveBeginPlay`
  (`KismetSystemLibrary.K2_SetTimerDelegate` (delegate `Hit Check`) 0.1 true)
  (`KismetSystemLibrary.Delay` 1.0)
  (`self.K2_DestroyActor`))

(event `Hit Check`
  (bind _returnvalue (`self.K2_GetActorLocation`))
  (bind _returnvalue_2 (`self.GetActorForwardVector`))
  (bind _hitdetectionline (`self.HitDetectionLine`))
  (bind _outhit (`KismetSystemLibrary.LineTraceSingle` (+ _returnvalue (* _returnvalue_2 _hitdetectionline)) (+ _returnvalue (* _returnvalue_2 (* _hitdetectionline -1.0))) "TraceTypeQuery1" false (`|MakeArray` (`self.GetOwner`))))
  (if (`KismetSystemLibrary.DoesImplementInterface` (`.HitActor` (`GameplayStatics.BreakHitResult` _outhit)) "/Game/Development/Davide/Interface/IF_ShotReaction.IF_ShotReaction_C")
    (message `/Game/Development/Davide/Interface/IF_ShotReaction.ShotReaction` (`.HitActor` (`GameplayStatics.BreakHitResult` _outhit)) (`self.GetOwner` self))
    (`self.K2_DestroyActor`)))

(fn `UserConstructionScript`)