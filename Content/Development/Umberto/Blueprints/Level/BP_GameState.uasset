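; Game state Blueprint that presents the end-of-level score screen and triggers the victory animation.
; DisplayScore adds ScoreWidget to the viewport, plays its intro animation and feeds it the final, time and target scores.
; The result of SetScore drives AnimPlay on the first BP_VIctoryAnimation actor found, then input switches to game-and-UI focused on the widget.
; TargetVanish is an empty event.
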(event `/Game/Development/Davide/Targets/IF_TargetManager.TargetVanish`)

(event `self.DisplayScore`
  (bind _scorewidget (`self.ScoreWidget`))
  (`UserWidget.AddToViewport` _scorewidget 0)
  (`|PlayAnimation2` _scorewidget (`/Game/Development/Umberto/Widget/WBP_ScoreScreen.ScoreScreenAnim` _scorewidget)
    (:`then`
      (bind _rank (`/Game/Development/Umberto/Widget/WBP_ScoreScreen.SetScore` _scorewidget (`KismetMathLibrary.Conv_IntToDouble` (`self.FinalScore`)) (`self.TimeScore`) (`self.TargetScore`)))
      (bind _outactors (`GameplayStatics.GetAllActorsOfClass` "/Game/Art/Axel/CustomAnimations/BP_VIctoryAnimation.BP_VIctoryAnimation_C"))
      (`/Game/Art/Axel/CustomAnimations/BP_VIctoryAnimation.AnimPlay` (`|GetArrayItem` _outactors) _rank)
      (`WidgetBlueprintLibrary.SetInputMode_GameAndUIEx` (`GameplayStatics.GetPlayerController` 0) _scorewidget))))

(fn `UserConstructionScript`)