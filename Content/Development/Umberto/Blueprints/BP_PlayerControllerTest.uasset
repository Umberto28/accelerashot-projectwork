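; Test player controller that routes Enhanced Input to the first-person test pawn for moving, looking and jumping.
; On BeginPlay it caches the BP_FirstPersonTest pawn and adds the default mapping context, then forwards input actions to that pawn.
; Move start, cancel and completion each toggle the pawn's IsRunning flag.
; Debug keys disable the game mode's tick, raise the pawn's top speed and toggle pause.
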(event `self.ReceiveBeginPlay`
  (bind _returnvalue (subsystem `EnhancedInputLocalPlayerSubsystem`))
  (bind _asbp_first_person_test (cast `/Game/Development/Umberto/Blueprints/BP_FirstPersonTest` (`GameplayStatics.GetPlayerPawn` 0)))
  (set `self.RefToPlayer` _asbp_first_person_test)
  (`/Engine/EditorBlueprintResources/StandardMacros.IsValid` _returnvalue
    (:`Is Valid`
      (`EnhancedInputSubsystemInterface.AddMappingContext` _returnvalue "/Game/Development/Umberto/Input/IMC_Default.IMC_Default" 0 (struct)))))

(event `EnhancedInput|/Game/Development/Umberto/Input/Actions/IA_Move`
  (params (ActionValue :type "Vector2D Structure") (ElapsedSeconds :type "Float (double-precision)") (TriggeredSeconds :type "Float (double-precision)") (InputAction :type "InputAction Object Reference" :default "/Game/Development/Umberto/Input/Actions/IA_Move.IA_Move"))
  (bind _reftoplayer (`self.RefToPlayer`))
  (:`Triggered`
    (`/Game/Development/Umberto/Blueprints/BP_FirstPersonTest.Move` (`self.RefToPlayer`) ActionValue_X ActionValue_Y))
  (:`Started`
    (bind _output_get (set `/Game/Development/Umberto/Blueprints/BP_FirstPersonTest.IsRunning` (not (`/Game/Development/Umberto/Blueprints/BP_FirstPersonTest.IsRunning` _reftoplayer)) _reftoplayer :!label _label))
    (`KismetSystemLibrary.PrintString` (`KismetStringLibrary.Conv_BoolToString` _output_get)))
  (:`Canceled`
    (goto _label))
  (:`Completed`
    (goto _label)))

(event `EnhancedInput|/Game/Development/Umberto/Input/Actions/IA_Jump`
  (params (ActionValue :type Boolean) (ElapsedSeconds :type "Float (double-precision)") (TriggeredSeconds :type "Float (double-precision)") (InputAction :type "InputAction Object Reference" :default "/Game/Development/Umberto/Input/Actions/IA_Jump.IA_Jump"))
  (bind _reftoplayer (`self.RefToPlayer`))
  (:`Started`
    (`Character.Jump` _reftoplayer))
  (:`Canceled`
    (`Character.StopJumping` _reftoplayer :!label _label_2))
  (:`Completed`
    (goto _label_2)))

(event `EnhancedInput|/Game/Development/Umberto/Input/Actions/IA_Look`
  (params (ActionValue :type "Vector2D Structure") (ElapsedSeconds :type "Float (double-precision)") (TriggeredSeconds :type "Float (double-precision)") (InputAction :type "InputAction Object Reference" :default "/Game/Development/Umberto/Input/Actions/IA_Look.IA_Look"))
  (:`Triggered`
    (`/Game/Development/Umberto/Blueprints/BP_FirstPersonTest.Aim` (`self.RefToPlayer`) ActionValue_X ActionValue_Y)))

(event `Key|R`
  (params (Key :type "Key Structure"))
  (:`Pressed`
    (`self.SetActorTickEnabled` (`GameplayStatics.GetGameMode`) false)))

(event `Key|C`
  (params (Key :type "Key Structure"))
  (bind _reftoplayer (`self.RefToPlayer`))
  (:`Pressed`
    (bind _output_get (set `/Game/Development/Umberto/Blueprints/BP_FirstPersonTest.TopSpeed` (+ (`/Game/Development/Umberto/Blueprints/BP_FirstPersonTest.TopSpeed` _reftoplayer) (`self.SpeedGain`)) _reftoplayer))
    (`KismetSystemLibrary.PrintString` (`KismetStringLibrary.Conv_DoubleToString` _output_get))))

(event `Key|P` :paused true
  (params (Key :type "Key Structure"))
  (:`Pressed`
    (`GameplayStatics.SetGamePaused` (not (`GameplayStatics.IsGamePaused`)))))

(fn `UserConstructionScript`)