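; Victory-animation Blueprint for the Axel character that drives the eye expression on its skeletal mesh.
; On BeginPlay it casts the mesh's anim instance to ABP_Axel and binds to its EyeChange dispatcher.
; Each dispatch passes the anim blueprint's Expression value to the "index" scalar of a dynamic eye material, created lazily on material slot zero and cached.
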(event `self.ReceiveBeginPlay`
  (bind _asabp_axel (cast `/Game/Art/Axel/CustomAnimations/ABP_Axel` (`SkeletalMeshComponent.GetAnimInstance` (`self.SkeletalMesh`)))
    (:`then`
      (add `/Game/Art/Axel/CustomAnimations/ABP_Axel.EyeChange` _asabp_axel (delegate `EyeChange_Event`)))
    (:`CastFailed`
      (`KismetSystemLibrary.PrintString` "Hello"))))

(event `EyeChange_Event`
  (`self.NotifyEyeChange` (`/Game/Art/Axel/CustomAnimations/ABP_Axel.Expression` (stale `self.ReceiveBeginPlay` _asabp_axel))))

(event `NotifyEyeChange`
  (params (ExpressionNum :type "Float (double-precision)"))
  (bind _eyeparam (`self.EyeParam`))
  (`/Engine/EditorBlueprintResources/StandardMacros.IsValid` _eyeparam
    (:`Is Valid`
      _)
    (:`Is Not Valid`
      (bind _returnvalue (`PrimitiveComponent.CreateDynamicMaterialInstance` (`self.SkeletalMesh`) 0 "/Game/Art/Axel/Materials/Eye1.Eye1" "None"))
      (set `self.EyeParam` _returnvalue)))
  (`MaterialInstanceDynamic.SetScalarParameterValue` _eyeparam "index" ExpressionNum))

(fn `UserConstructionScript`)