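; Weapon component, apparently for a first-person character, that tracks a bullet count with manual and target-triggered reloading.
; ManualReload flags reloading, prints a message, waits ReloadTime and refills to a fixed count, while TargetReload adds one bullet.
; The shooting chain, which spawns BP_BaseBullet along the owner's camera or reloads when empty, is disconnected from the empty IA_Shoot event, so it never runs.
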(event `EnhancedInput|/Game/Development/Davide/Shooting/IA_Shoot`
  (params (ActionValue :type Boolean) (ElapsedSeconds :type "Float (double-precision)") (TriggeredSeconds :type "Float (double-precision)") (InputAction :type "InputAction Object Reference" :default "/Game/Development/Davide/Shooting/IA_Shoot.IA_Shoot"))
  ; Ammunition Check
)

(event `TargetReload`
  ; Target Reload
  (`/Engine/EditorBlueprintResources/StandardMacros.IncrementInt` (`self.BulletNumber`)))

(event `ManualReload`
  ; Manual Reload
  (`self.IsReloading`
    (:`then`)
    (:`else`
      (set `self.IsReloading` true)
      (`KismetSystemLibrary.PrintString` "Reloading...")
      (`KismetSystemLibrary.Delay` (`self.ReloadTime`))
      (set `self.IsReloading` false)
      (set `self.BulletNumber` 3))))