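; BP_AxelBox is a main menu box with widget screens on its front, right, left and back faces.
; Its OnScreenChange event takes active and inactive indices and maps each to a face's widget.
; The active widget becomes Visible and the inactive one HitTestInvisible, so it still renders but ignores pointer input.
; The construction script is empty and the file contains no rotation logic.
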(event `OnScreenChange`
  (params (ActiveIdx :type Integer) (InactiveIdx :type Integer))
  (bind _returnvalue (`WidgetComponent.GetWidget` (`self.BoxFront`)))
  (bind _returnvalue_2 (`WidgetComponent.GetWidget` (`self.BoxRight`)))
  (bind _returnvalue_3 (`WidgetComponent.GetWidget` (`self.BoxLeft`)))
  (bind _returnvalue_4 (`WidgetComponent.GetWidget` (`self.BoxBack`)))
  (`Widget.SetVisibility` (select `int` ActiveIdx :`0` _returnvalue :`1` _returnvalue_2 :`2` _returnvalue_3 :`3` _returnvalue_4) "Visible")
  (`Widget.SetVisibility` (select `int` InactiveIdx :`0` _returnvalue :`1` _returnvalue_2 :`2` _returnvalue_3 :`3` _returnvalue_4) "HitTestInvisible"))

(fn `UserConstructionScript`)