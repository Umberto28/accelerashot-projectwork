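; BP_BaseTarget is a shootable target that rewards the shooter with speed and ammo.
; ShotReaction casts the bullet owner to BP_FirstPersonTest, grants SpeedGain through GainSpeed, and calls TargetReload on its hitscan weapon component.
; It then calls Vanish, which hides the root and its children; a separate Restore event makes them visible again, toggling visibility only, without destroying the actor.
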(event `/Game/Development/Davide/Interface/IF_ShotReaction.ShotReaction`
  (params (BulletOwner :type "Actor Object Reference"))
  ; Player gains speed and a bullet from the hit
  (bind _asbp_first_person_test (cast `/Game/Development/Umberto/Blueprints/BP_FirstPersonTest` BulletOwner))
  (`/Game/Development/Umberto/Blueprints/BP_FirstPersonTest.GainSpeed` _asbp_first_person_test (`self.Speed Gain`))
  (`/Game/Development/Davide/BPC_HitscanWeapon.TargetReload` (`/Game/Development/Umberto/Blueprints/BP_FirstPersonTest.BPC_HitscanWeapon` _asbp_first_person_test))
  (`self.Vanish`))

(event `Vanish`
  ; Make Targets Vanish and Reappear
  (`SceneComponent.SetVisibility` (`self.DefaultSceneRoot`) false true))

(event `Restore`
  ; Make Targets Vanish and Reappear
  (`SceneComponent.SetVisibility` (`self.DefaultSceneRoot`) true true))

(fn `UserConstructionScript`)