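; Base shootable target that rewards the player with a speed gain and a weapon reload when shot on a component tagged TTarget.
; On a valid hit it hides its root hierarchy and fires OnTargetVanish.
; At BeginPlay it binds to the game mode's OnTargetsReset and its own vanish dispatcher, with a restore event to show it again.
; The construction script destroys the movement and shooter components that TargetType does not enable.
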(event `self.ReceiveBeginPlay`
  (bind _aslevel_game_mode (cast `LevelGameMode` (`GameplayStatics.GetGameMode`)))
  (bind _output_get (set `self.RefToGameMode` _aslevel_game_mode))
  (add `LevelGameMode.OnTargetsReset` _output_get (`|CreateDelegate` :!event `TargetRestore`))
  ; Sends delegate to component by event name
  (add `LevelGameMode.OnTargetsReset` _output_get (`|CreateDelegate` (`self.BPC_TargetShooter`) :!event `Restore`))
  (add `self.OnTargetVanish` (`|CreateDelegate` (`self.BPC_TargetShooter`) :!event `Vanish`)))

(event `/Game/Development/Davide/Interface/IF_ShotReaction.ShotReaction`
  (params (BulletOwner :type "Actor Object Reference") (HitComponent :type "ActorComponent Object Reference"))
  ; Player gains speed and a bullet from the hit
  (if (`ActorComponent.ComponentHasTag` HitComponent "TTarget")
    (bind _asbp_first_person_test (cast `/Game/Development/Umberto/Blueprints/BP_FirstPersonTest` BulletOwner))
    (`/Game/Development/Umberto/Blueprints/BP_FirstPersonTest.GainSpeed` _asbp_first_person_test (`self.SpeedGain`))
    (`/Game/Development/Davide/Shooting/BPC_HitscanWeapon.TargetReload` (`/Game/Development/Umberto/Blueprints/BP_FirstPersonTest.BPC_HitscanWeapon` _asbp_first_person_test))
    (`self.Vanish`)
    (`self.OnTargetVanish`)))

(event `Vanish`
  ; Make Targets Vanish and Reappear
  (`SceneComponent.SetVisibility` (`self.DefaultSceneRoot`) false true))

(event `TargetRestore`
  ; Make Targets Vanish and Reappear
  (`SceneComponent.SetVisibility` (`self.DefaultSceneRoot`) true true))

(fn `UserConstructionScript`
  (bind (_targettype_moving _targettype_shooting) (break `/Game/Development/Davide/Targets/S_TargetTypes` (`self.TargetType`)))
  (if (not _targettype_moving)
    (`ActorComponent.K2_DestroyComponent` (`self.BPC_TargetMovement`)))
  (if (not _targettype_shooting)
    (`ActorComponent.K2_DestroyComponent` (`self.BPC_TargetShooter`))))