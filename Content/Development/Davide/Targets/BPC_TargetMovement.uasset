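; Actor component that moves its owning target back and forth in a sine oscillation around its starting location.
; BeginPlay caches the owner and its base location, then Tick offsets it along the owner's up and right vectors by a time-based sine scaled by speed and a 2D length.
; Interface events for target vanish and reset switch the component's tick off and on.
; An unused spline-path alternative remains disconnected.
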(event `self.ReceiveBeginPlay`
  (bind _output_get (set `self.RefToOwner` (`self.GetOwner`)))
  (set `self.BaseLocation` (`Actor.K2_GetActorLocation` _output_get)))

(event `self.ReceiveTick`
  (params (DeltaSeconds :type "Float (single-precision)"))
  (bind _reftoowner (`self.RefToOwner`))
  (bind (_returnvalue_x _returnvalue_y) (`KismetMathLibrary.BreakVector2D` (* (`KismetMathLibrary.Sin` (* (`GameplayStatics.GetTimeSeconds`) (`self.Speed`))) (`self.Length2D`))))
  (`Actor.K2_SetActorLocation` (`self.RefToOwner`) (+ (`self.BaseLocation`) (* (`Actor.GetActorUpVector` _reftoowner) _returnvalue_x) (* (`Actor.GetActorRightVector` _reftoowner) _returnvalue_y)) false false))

(event `/Game/Development/Davide/Targets/IF_TargetManager.TargetVanish`
  ; Vanish or restore with target (interfaces)
  (`self.SetComponentTickEnabled` false))

(event `/Game/Development/Davide/Targets/IF_TargetManager.TargetReset`
  ; Vanish or restore with target (interfaces)
  (`self.SetComponentTickEnabled` true))