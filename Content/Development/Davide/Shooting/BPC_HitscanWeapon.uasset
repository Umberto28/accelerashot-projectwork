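; Scene component for a hitscan weapon with limited ammo, firing instant line traces along its forward vector.
; Shooting spends a bullet and traces on the Visibility channel with debug drawing, sending ShotReactionMessage with owner and hit component to actors implementing IF_ShotReaction.
; An empty magazine triggers ManualReload, which resets the bullet count to a fixed amount after ReloadTime.
; TargetReload separately adds one bullet immediately.
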(event `Shooting`
  (bind _returnvalue (`self.K2_GetComponentLocation` self))
  ; Ammunition Check
  (if (> (`self.BulletNumber`) 0)
    ; Shooting
    (`/Engine/EditorBlueprintResources/StandardMacros.DecrementInt` (`self.BulletNumber`)
      (:`  `
        (bind _outhit (`KismetSystemLibrary.LineTraceSingle` :`Start` _returnvalue :`End` (+ _returnvalue (* (`self.GetForwardVector` self) (`self.Range`))) :`TraceChannel` "TraceTypeQuery1" :`DrawDebugType` "ForDuration"))
        (if (`KismetSystemLibrary.DoesImplementInterface` (`.HitActor` (`GameplayStatics.BreakHitResult` _outhit)) "/Game/Development/Davide/Interface/IF_ShotReaction.IF_ShotReaction_C")
          (message `/Game/Development/Davide/Interface/IF_ShotReaction.ShotReaction` (`.HitActor` (`GameplayStatics.BreakHitResult` _outhit)) (`self.GetOwner` self) (`.HitComponent` (`GameplayStatics.BreakHitResult` _outhit))))))
    (else
      ;; Must Reload
      (`self.ManualReload`))))

(event `TargetReload`
  ; Target Reload
  (`/Engine/EditorBlueprintResources/StandardMacros.IncrementInt` (`self.BulletNumber`)))

(event `ManualReload`
  ; Manual Reload
  (`KismetSystemLibrary.PrintString` "Reloading...")
  (`KismetSystemLibrary.Delay` (`self.ReloadTime`))
  (set `self.BulletNumber` 3))