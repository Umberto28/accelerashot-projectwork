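; Weapon component for the first-person test character that handles shooting and ammunition.
; The shoot input spends a bullet and spawns a BP_BaseBullet at the owner's camera, aimed along its forward vector, or triggers a manual reload when empty.
; Manual reload is guarded by a reloading flag and resets the count after a delay.
; A separate TargetReload event adds one bullet instantly, with no cap.
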(event `EnhancedInput|/Game/Development/Davide/IA_Shoot`
  (params (ActionValue :type Boolean) (ElapsedSeconds :type "Float (double-precision)") (TriggeredSeconds :type "Float (double-precision)") (InputAction :type "InputAction Object Reference" :default "/Game/Development/Davide/IA_Shoot.IA_Shoot"))
  (bind _returnvalue (`self.GetOwner`))
  ; Ammunition Check
  (:`Started`
    (if (> (`self.BulletNumber`) 0)
      ; Shooting
      (`/Engine/EditorBlueprintResources/StandardMacros.DecrementInt` (`self.BulletNumber`)
        (:`  `
          (bind _asbp_first_person_test (cast `/Game/Development/Umberto/Blueprints/BP_FirstPersonTest` _returnvalue))
          (bind _camera (`/Game/Development/Umberto/Blueprints/BP_FirstPersonTest.Camera` _asbp_first_person_test))
          (`|SpawnActorFromClass` "/Game/Development/Davide/BP_BaseBullet.BP_BaseBullet_C" (`KismetMathLibrary.MakeTransform` (`SceneComponent.K2_GetComponentLocation` _camera) (`KismetMathLibrary.Conv_VectorToRotator` (`SceneComponent.GetForwardVector` _camera))) "AlwaysSpawn" "MultiplyWithRoot" _returnvalue null)))
      (else
        ; Must Reload
        (`self.ManualReload`)))))

(event `TargetReload`
  ; Target Reload
  (`/Engine/EditorBlueprintResources/StandardMacros.IncrementInt` (`self.BulletNumber`)))

(event `ManualReload`
  ; Manual Reload
  (`self.IsReloading`
    (:`then`)
    (:`else`
      (set `self.IsReloading` true)
      (`KismetSystemLibrary.PrintString` "Reloading...")
      (`KismetSystemLibrary.Delay` (`self.ReloadTime`))
      (set `self.IsReloading` false)
      (set `self.BulletNumber` 3))))