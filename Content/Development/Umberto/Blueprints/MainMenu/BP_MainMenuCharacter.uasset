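; Main menu character that slides along the spline on BP_AxelBox when the menu index changes.
; OnIndexChange derives a left or right direction from the index delta and stores the target point's location.
; Each timeline update nudges the actor that way, snaps it to the nearest spline location and turns it to face the box.
; The stored target and timeline output don't drive the movement, and the current index is never updated here.
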(event `self.ReceiveBeginPlay`
  (bind _returnvalue (`GameplayStatics.GetActorOfClass` "/Game/Development/Umberto/Blueprints/MainMenu/BP_AxelBox.BP_AxelBox_C"))
  (set `self.RefToAxelBox` _returnvalue))

(event `OnIndexChange`
  (params (NewIdx :type Integer))
  (bind _currsplineidx (`self.CurrSplineIdx`))
  (if (!= NewIdx _currsplineidx)
    (set `self.NextDirection` (* (`self.GetActorRightVector`) (`KismetMathLibrary.SignOfInteger` (- NewIdx _currsplineidx))))
    (set `self.CurrTargetLocation` (`SplineComponent.GetLocationAtSplinePoint` (`/Game/Development/Umberto/Blueprints/MainMenu/BP_AxelBox.Spline` (`self.RefToAxelBox`)) NewIdx "World"))
    (`Timeline|TransformTimeline` :!via `PlayFromStart`
      (:`Update`
        (`|ExecutionSequence`
          (:`then_0`
            (`self.K2_SetActorLocation` (`SplineComponent.FindLocationClosestToWorldLocation` (`/Game/Development/Umberto/Blueprints/MainMenu/BP_AxelBox.Spline` (`self.RefToAxelBox`)) (+ (`self.K2_GetActorLocation`) (`self.NextDirection`)) "World")))
          (:`then_1`
            (`self.K2_SetActorRotation` (`KismetMathLibrary.FindLookAtRotation` (`self.K2_GetActorLocation`) (`self.K2_GetActorLocation` (`self.RefToAxelBox`))))))))))

(fn `UserConstructionScript`
  (`self.K2_SetActorRotation` (struct :`Pitch` -25.0 :`Yaw` 90.0)))