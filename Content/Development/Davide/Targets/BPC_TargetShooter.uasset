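; BPC_TargetShooter is an actor component that makes its owner fire bullets at the player.
; On BeginPlay it starts a looping timer at RateOfFire that calls Shoot.
; While IsActivated is true, each shot spawns a BP_BaseBullet at the owner's location, rotated toward player pawn 0 and owned by that actor.
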(event `self.ReceiveBeginPlay`
  (set `self.RefToOwner` (`self.GetOwner`))
  (`KismetSystemLibrary.K2_SetTimerDelegate` (delegate `Shoot`) (`self.RateOfFire`) true true))

(event `Shoot`
  (bind _returnvalue (`Actor.K2_GetActorLocation` (`self.RefToOwner`)))
  (if (`self.IsActivated`)
    (bind _output_get (set `self.BulletTransform` (`KismetMathLibrary.MakeTransform` _returnvalue (`KismetMathLibrary.FindLookAtRotation` _returnvalue (`Actor.K2_GetActorLocation` (`GameplayStatics.GetPlayerPawn` 0))))))
    (`|SpawnActorFromClass` "/Game/Development/Davide/Shooting/BP_BaseBullet.BP_BaseBullet_C" _output_get "Undefined" "MultiplyWithRoot" (`self.GetOwner`) null)))