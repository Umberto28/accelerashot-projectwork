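; Level game mode for a timed target-hitting level, tracking targets hit and elapsed time.
; BeginPlay creates the level HUD and caches every BP_BaseTarget actor and their total.
; Tick accumulates delta time, passes whole seconds and hundredths through a timespan, and writes the formatted timestamp straight to the HUD.
; UpdateTargetCount increments hits, while RestoreTargets zeroes hits and timer and restores every cached target.
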(event `self.ReceiveBeginPlay`
  (bind _returnvalue (`|CreateWidget` "/Game/Development/Umberto/Widget/WBP_LevelHUD.WBP_LevelHUD_C"))
  (bind _output_get (set `self.RefToHUD` _returnvalue))
  (`UserWidget.AddToViewport` _output_get 0)
  (bind _outactors (`GameplayStatics.GetAllActorsOfClass` "/Game/Development/Davide/BP_BaseTarget.BP_BaseTarget_C"))
  (bind _output_get_2 (set `self.RefToTargets` _outactors))
  (set `self.TotalTargets` (`KismetArrayLibrary.Array_Length` _output_get_2)))

(event `self.ReceiveTick`
  (params (DeltaSeconds :type "Float (single-precision)"))
  (bind _output_get (set `self.TimeValue` (+ DeltaSeconds (`self.TimeValue`))))
  (bind _returnvalue (`KismetMathLibrary.FTrunc` _output_get))
  (bind (_days _hours _minutes _seconds _milliseconds) (`KismetMathLibrary.BreakTimespan` (`KismetMathLibrary.MakeTimespan` 0 0 0 _returnvalue (`KismetMathLibrary.FTrunc` (* (- _output_get _returnvalue) 100.0)))))
  (bind _output_get_2 (set `self.TimeStamp` (`|FormatText` "{h}:{min}:{s}:{milli}" (`KismetTextLibrary.Conv_IntToText` _hours false true 2) (`KismetTextLibrary.Conv_IntToText` _minutes false true 2) (`KismetTextLibrary.Conv_IntToText` _seconds false true 2) (`KismetTextLibrary.Conv_IntToText` _milliseconds false true 2))))
  (set `TextBlock.Text` _output_get_2 (`/Game/Development/Umberto/Widget/WBP_LevelHUD.TimeStampText` (`self.RefToHUD`))))

(fn `RestoreTargets`
  (set `self.TargetsHit` 0)
  (set `self.TimeValue` 0.0)
  (for _array_element (`self.RefToTargets`)
    (`/Game/Development/Davide/BP_BaseTarget.Restore` _array_element)))

(fn `UpdateTargetCount`
  (`/Engine/EditorBlueprintResources/StandardMacros.IncrementInt` (`self.TargetsHit`)))

(fn `UserConstructionScript`)