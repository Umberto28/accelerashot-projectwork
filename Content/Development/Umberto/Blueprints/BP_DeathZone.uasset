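; BP_DeathZone is a kill volume that fails the player on contact.
; When DeathCollision begins overlapping a BP_FirstPersonTest, it calls that character's Failure function.
; BeginPlay caches the player's starting location, control rotation and the BP_LevelGameMode reference.
; A ResetPlayerState function can restore that location and rotation, but nothing in this Blueprint calls it or uses the game mode reference.
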(event `self.ReceiveBeginPlay`
  (bind _returnvalue (`GameplayStatics.GetPlayerPawn` 0))
  (set `self.StartingLocation` (`self.K2_GetActorLocation` _returnvalue))
  (set `self.StartingRotation` (`Pawn.GetControlRotation` _returnvalue))
  (bind _asbp_level_game_mode (cast `/Game/Development/Umberto/Blueprints/BP_LevelGameMode` (`GameplayStatics.GetGameMode`)))
  (set `self.RefToGameMode` _asbp_level_game_mode))

(event `self.DeathCollision.OnComponentBeginOverlap`
  (params (OverlappedComponent :type "PrimitiveComponent Object Reference") (OtherActor :type "Actor Object Reference") (OtherComp :type "PrimitiveComponent Object Reference") (OtherBodyIndex :type Integer) (bFromSweep :type Boolean) (SweepResult :type "HitResult Structure (by ref)"))
  (bind _asbp_first_person_test (cast `/Game/Development/Umberto/Blueprints/BP_FirstPersonTest` OtherActor))
  (`/Game/Development/Umberto/Blueprints/BP_FirstPersonTest.Failure` _asbp_first_person_test))

(fn `ResetPlayerState`
  (params (Player :type "Pawn Object Reference"))
  (`self.K2_SetActorLocation` Player (`self.StartingLocation`) false false)
  (`Controller.SetControlRotation` (`Pawn.GetController` Player) (`self.StartingRotation`)))

(fn `UserConstructionScript`)