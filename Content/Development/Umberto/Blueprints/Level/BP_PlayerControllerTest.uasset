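; Test player controller that caches the BP_FirstPersonTest pawn on BeginPlay and forwards Enhanced Input move, look, jump and shoot actions to it.
; Move input also sets the pawn's IsRunning flag from a horizontal speed threshold.
; The pause action either pauses the game and calls OnGamePaused, or resumes through the pause widget.
; Hardcoded keys disable game mode ticking (R) and grant the player speed (C).
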(event `self.ReceiveBeginPlay`
  (bind _asbp_first_person_test (cast `/Game/Development/Umberto/Blueprints/Level/BP_FirstPersonTest` (`GameplayStatics.GetPlayerPawn` 0)))
  (set `self.RefToPlayer` _asbp_first_person_test))

(event `EnhancedInput|/Game/Development/Umberto/Input/Actions/IA_Move`
  (params (ActionValue :type "Vector2D Structure") (ElapsedSeconds :type "Float (double-precision)") (TriggeredSeconds :type "Float (double-precision)") (InputAction :type "InputAction Object Reference" :default "/Game/Development/Umberto/Input/Actions/IA_Move.IA_Move"))
  (bind _reftoplayer (`self.RefToPlayer`))
  ; Movement
  (:`Triggered`
    ;; When in the character considered as moving?
    (if (> (`KismetMathLibrary.VSizeXY` (`self.GetVelocity` _reftoplayer)) 255.0)
      (set `/Game/Development/Umberto/Blueprints/Level/BP_FirstPersonTest.IsRunning` true _reftoplayer)
      (else
        (set `/Game/Development/Umberto/Blueprints/Level/BP_FirstPersonTest.IsRunning` false _reftoplayer)))
    (`/Game/Development/Umberto/Blueprints/Level/BP_FirstPersonTest.Move` _reftoplayer ActionValue_X ActionValue_Y)))

(event `EnhancedInput|/Game/Development/Umberto/Input/Actions/IA_Look`
  (params (ActionValue :type "Vector2D Structure") (ElapsedSeconds :type "Float (double-precision)") (TriggeredSeconds :type "Float (double-precision)") (InputAction :type "InputAction Object Reference" :default "/Game/Development/Umberto/Input/Actions/IA_Look.IA_Look"))
  ; Aiming & Shooting
  (:`Triggered`
    (`/Game/Development/Umberto/Blueprints/Level/BP_FirstPersonTest.Aim` (`self.RefToPlayer`) ActionValue_X ActionValue_Y)))

(event `EnhancedInput|/Game/Development/Umberto/Input/Actions/IA_Jump`
  (params (ActionValue :type Boolean) (ElapsedSeconds :type "Float (double-precision)") (TriggeredSeconds :type "Float (double-precision)") (InputAction :type "InputAction Object Reference" :default "/Game/Development/Umberto/Input/Actions/IA_Jump.IA_Jump"))
  (bind _reftoplayer (`self.RefToPlayer`))
  ; Jumping
  (:`Started`
    (`Character.Jump` _reftoplayer))
  (:`Canceled`
    (`Character.StopJumping` _reftoplayer :!label _label))
  (:`Completed`
    (goto _label)))

(event `EnhancedInput|/Game/Development/Davide/Shooting/IA_Shoot`
  (params (ActionValue :type Boolean) (ElapsedSeconds :type "Float (double-precision)") (TriggeredSeconds :type "Float (double-precision)") (InputAction :type "InputAction Object Reference" :default "/Game/Development/Davide/Shooting/IA_Shoot.IA_Shoot"))
  ; Aiming & Shooting
  (:`Started`
    (`/Game/Development/Umberto/Blueprints/Level/BP_FirstPersonTest.Shoot` (`self.RefToPlayer`))))

(event `Key|R`
  (params (Key :type "Key Structure"))
  (:`Pressed`
    (`self.SetActorTickEnabled` (`GameplayStatics.GetGameMode`) false)))

(event `Key|C`
  (params (Key :type "Key Structure"))
  (:`Pressed`
    (`/Game/Development/Umberto/Blueprints/Level/BP_FirstPersonTest.GainSpeed` (`self.RefToPlayer`) 400.0)))

(event `EnhancedInput|/Game/Development/Umberto/Input/Actions/IA_Pause`
  (params (ActionValue :type Boolean) (ElapsedSeconds :type "Float (double-precision)") (TriggeredSeconds :type "Float (double-precision)") (InputAction :type "InputAction Object Reference" :default "/Game/Development/Umberto/Input/Actions/IA_Pause.IA_Pause"))
  ; Pausing
  (:`Started`
    (if (`GameplayStatics.IsGamePaused`)
      (`PauseMenuWidget.OnResumeClicked` (`self.WidgetPause`))
      (else
        (`self.SetPauseGame`)
        (`self.OnGamePaused` true)))))

(fn `UserConstructionScript`)